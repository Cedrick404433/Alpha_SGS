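; GM_Main is a game mode Blueprint that runs a minutes and seconds countdown.
; BeginPlay prints an activation message and starts a looping one-second timer, apparently bound to E_Timer, which decrements Seconds and rolls over into Minutes.
; The greater-or-equal-to-zero checks let both values drop below zero.
; A check for both reaching zero is unconnected, so nothing ends the countdown.
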(event `self.ReceiveBeginPlay`
  (`KismetSystemLibrary.PrintString` "Gamemode Active" true true (struct :`G` 1.0 :`A` 1.0))
  (`KismetSystemLibrary.K2_SetTimerDelegate` (`|CreateDelegate` :!event `E_Timer`) 1.0 true))

(event `E_Timer`
  (if (>= (`self.Seconds`) 0)
    (bind _result (`/Engine/EditorBlueprintResources/StandardMacros.DecrementInt` (`self.Seconds`))
      (:`  `
        (set `self.Seconds` _result)))
    (elif (>= (`self.Minutes`) 0)
      (`/Engine/EditorBlueprintResources/StandardMacros.DecrementInt` (`self.Minutes`)
        (:`  `
          (set `self.Seconds` 59)))
      (else
        (bind _result_2 (`/Engine/EditorBlueprintResources/StandardMacros.DecrementInt` (`self.Seconds`))
          (:`  `
            (set `self.Seconds` _result_2)))))))

(fn `UserConstructionScript`)