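; Camera Blueprint that pans between preset positions in response to left, right and down move events.
; Left and right step a numeric row name with wraparound between min and max, while down always selects row 0.
; The row's location and rotation from DT_CameraPositions drive MoveComponentTo.
; Before non-down moves, a near-instant yaw nudge biases the shortest-path blend toward the intended pan direction.
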(event `ce_leftCamera`
  (bind _returnvalue (`self.GetComponentByClass` "/Script/Engine.SceneComponent"))
  (bind (_returnvalue_roll _returnvalue_pitch _returnvalue_yaw) (`KismetMathLibrary.BreakRotator` (`self.K2_GetActorRotation`)))
  ;[0 1 0.0832] Event called when camera is to move, either via key or button press. Checks if camera is already moving, and then which direction it should move.
  (if (not (`self.IsCameraMoving?`))
    (set `self.isCameraMovingLeft?` true)
    ;[0 1 0.0832] Does calculations based on the min and max cameras (how many cameras we have) and which direction its moving to determine which one it needs to swap to.
    (bind _result (`/Engine/EditorBlueprintResources/StandardMacros.IncrementInt` (`KismetStringLibrary.Conv_StringToInt` (`KismetStringLibrary.Conv_NameToString` (`self.currentCameraRow`))))
      (:`  `
        (if (> _result (`self.maxCamera`))
          (set `self.currentCameraInt` (`self.minCamera`))
          (else
            (set `self.currentCameraInt` _result)))
        (bind _output_get (set `self.currentCameraRow` (`KismetStringLibrary.Conv_StringToName` (`KismetStringLibrary.Conv_IntToString` (`self.currentCameraInt`))) :!label _label))
        ;[0 1 0.0832] Pulls the required information from the DT_CameraPos for the camera we're moving to, also sets the camera moving bool.
        (bind _returnvalue_2 (`|GetDataTableRow` "/Game/Blueprints/Datatables/DT_CameraPositions.DT_CameraPositions" _output_get :!label _label_2)
          (:`then`
            (set `self.Out Row Camera Location` (`.cameraLocation_7_C21CEA024EC41D94D6527B98BE0FC170` (break `/Game/Blueprints/Datatables/STR_Camera` _returnvalue_2)))
            (set `self.Out Row Camera Rotation` (`.cameraRotation_8_F37565CC4CD6D19809EC77B7E887FE10` (break `/Game/Blueprints/Datatables/STR_Camera` _returnvalue_2)))
            (set `self.IsCameraMoving?` true)
            ;[0 1 0.0832] Uses the camera moving direction to branch.
            (if (not (`self.isCameraMovingDown?`))
              (if (`self.isCameraMovingLeft?`)
                ;[0 1 0.0832] Uses cameras current rotation + intended moving direction, then bumps the camera slightly in that direction, thereby changing the optimal route the blend takes ahead of the next blend, making the camera always pan in the correct direction.
                (set `self.tempYaw` (- _returnvalue_yaw 10.0))
                (else
                  (set `self.tempYaw` (+ _returnvalue_yaw 10.0))))
              (`KismetSystemLibrary.MoveComponentTo` _returnvalue (`self.Out Row Camera Location`) (`KismetMathLibrary.MakeRotator` _returnvalue_roll _returnvalue_pitch (`self.tempYaw`)) false false 0.01 true))
            ;[0 1 0.0832] Moves camera to new location, then resets bools.
            (`KismetSystemLibrary.MoveComponentTo` _returnvalue (`self.Out Row Camera Location`) (`self.Out Row Camera Rotation`) false false 0.2 true)
            (set `self.IsCameraMoving?` false)
            (set `self.isCameraMovingLeft?` false)
            (set `self.isCameraMovingDown?` false)))))))

(event `ce_rightCamera`
  ;[0 1 0.0832] Event called when camera is to move, either via key or button press. Checks if camera is already moving, and then which direction it should move.
  ;[0 1 0.0832] Does calculations based on the min and max cameras (how many cameras we have) and which direction its moving to determine which one it needs to swap to.
  (bind _result (`/Engine/EditorBlueprintResources/StandardMacros.DecrementInt` (`KismetStringLibrary.Conv_StringToInt` (`KismetStringLibrary.Conv_NameToString` (`self.currentCameraRow`))))
    (:`  `
      (if (< _result (`self.minCamera`))
        (set `self.currentCameraInt` (`self.maxCamera`))
        (goto _label)
        (else
          (set `self.currentCameraInt` _result)
          (goto _label))))))

(event `ce_downCamera`
  ;[0 1 0.0832] Event called when camera is to move, either via key or button press. Checks if camera is already moving, and then which direction it should move.
  (if (not (`self.IsCameraMoving?`))
    (set `self.isCameraMovingDown?` true)
    ;[0 1 0.0832] Always sets the camera to the same one when moving 'down'.
    (set `self.currentCameraRow` "0")
    (goto _label_2)))

(fn `UserConstructionScript`)