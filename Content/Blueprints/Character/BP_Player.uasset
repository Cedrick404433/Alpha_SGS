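; BP_Player is the player Blueprint that sets up the in-game UI and handles pausing.
; On BeginPlay it shows the mouse cursor and, outside L_MainMenu, adds the HUD widget and caches a reference to the Bp_camera actor.
; P and Escape share one path that creates the pause menu widget, adds it to the viewport and pauses the game.
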(event `Key|P`
  (params (Key :type "Key Structure"))
  (:`Pressed`
    (bind _returnvalue (`|CreateWidget` "/Game/UI/WBP_PauseMenu.WBP_PauseMenu_C" (`GameplayStatics.GetPlayerController` 0) :!label _label))
    (bind _output_get (set `self.Ref_WBP_PauseMenu` _returnvalue))
    (`UserWidget.AddToViewport` _output_get 0)
    (`GameplayStatics.SetGamePaused` true)))

(event `Key|Escape`
  (params (Key :type "Key Structure"))
  (:`Pressed`
    (goto _label)))

(event `self.ReceiveBeginPlay`
  ;[0.3437 0 1] Inside PlayerController - Set Enable Click Event 'True'
  (set `PlayerController.bShowMouseCursor` true (`GameplayStatics.GetPlayerController` 0))
  (`KismetSystemLibrary.PrintString` "Show")
  (bind _returnvalue (`GameplayStatics.GetCurrentLevelName` true))
  (if (not (`KismetStringLibrary.EqualEqual_StrStr` _returnvalue "L_MainMenu"))
    (bind _returnvalue_2 (`|CreateWidget` "/Game/UI/WBP_HUD.WBP_HUD_C" (`GameplayStatics.GetPlayerController` 0)))
    (bind _output_get (set `self.Ref_HUD` _returnvalue_2))
    (`UserWidget.AddToViewport` _output_get 0)
    (bind _returnvalue_3 (`GameplayStatics.GetActorOfClass` "/Game/Blueprints/Character/bp_camera.bp_camera_C"))
    (set `self.Ref_Cam` _returnvalue_3)))

(fn `UserConstructionScript`)