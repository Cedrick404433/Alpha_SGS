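; BP_Potion is a clickable potion pickup actor that the player can collect.
; It caches the BP_Player character on BeginPlay, and clicking its cube checks that the player holds neither an ingredient nor another potion.
; If both hands are free, it flags the potion as held on the player, destroys itself and sets its icon on the HUD item box.
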(event `self.ReceiveBeginPlay`
  ;[0 0.04314 1] Casting
  (bind _asbp_player (cast `/Game/Blueprints/Character/BP_Player` (`GameplayStatics.GetPlayerCharacter` 0)))
  (set `self.Ref_Player` _asbp_player))

(event `self.Cube.OnClicked`
  (params (TouchedComponent :type "PrimitiveComponent Object Reference") (ButtonPressed :type "Key Structure"))
  ;[0 0.04314 1] Pickup
  (if (not (`/Game/Blueprints/Character/BP_Player.IngredientHeld?` (`self.Ref_Player`)))
    (if (not (`/Game/Blueprints/Character/BP_Player.IsPotionHeld?` (`self.Ref_Player`)))
      (set `/Game/Blueprints/Character/BP_Player.IsPotionHeld?` true (`self.Ref_Player`))
      (`self.K2_DestroyActor`)
      (`Image.SetBrushFromTexture` (`/Game/UI/WBP_HUD.Img_ItemBox` (`/Game/Blueprints/Character/BP_Player.Ref_HUD` (`self.Ref_Player`))) (`self.Icon`) false))))

(fn `UserConstructionScript`)