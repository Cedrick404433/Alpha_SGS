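; BP_Ingredient is a clickable world ingredient that the player can pick up, one at a time.
; Clicking plays a sound and, if the player holds neither ingredient nor potion, records the ingredient's name on BP_Player and puts its icon in the HUD item box.
; Hovering shows a name label, filled by the construction script, and applies a yellow overlay highlight.
; The actor stays in place after pickup.
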(event `self.ReceiveBeginPlay`
  ;[0 0.003347 1] Casting
  (bind _asbp_player (cast `/Game/Blueprints/Character/BP_Player` (`GameplayStatics.GetPlayerCharacter` 0)))
  (set `self.Ref_Player` _asbp_player))

(event `self.SM_Main.OnClicked`
  (params (TouchedComponent :type "PrimitiveComponent Object Reference") (ButtonPressed :type "Key Structure"))
  (bind _ref_player (`self.Ref_Player`))
  ;[0 0.04314 1] Ingredient Pickup
  (`GameplayStatics.PlaySound2D` "/Game/Placeholder/Audio/SW_WaterDrop.SW_WaterDrop" 1.0 1.0 0.0 null null)
  (if (not (`/Game/Blueprints/Character/BP_Player.IngredientHeld?` (`self.Ref_Player`)))
    (if (not (`/Game/Blueprints/Character/BP_Player.IsPotionHeld?` (`self.Ref_Player`)))
      (set `/Game/Blueprints/Character/BP_Player.IngredientHeld?` true _ref_player)
      (bind _output_get (set `/Game/Blueprints/Character/BP_Player.IngredientName` (`self.Name`) _ref_player))
      (`KismetSystemLibrary.PrintString` (`KismetStringLibrary.Concat_StrStr` "Picked up " (`KismetStringLibrary.Conv_NameToString` _output_get)))
      (`Image.SetBrushFromTexture` (`/Game/UI/WBP_HUD.Img_ItemBox` (`/Game/Blueprints/Character/BP_Player.Ref_HUD` (`self.Ref_Player`))) (`self.Icon`) false))
    (else
      (`KismetSystemLibrary.PrintString` "Ingredient Already Held"))))

(event `self.SM_Main.OnBeginCursorOver`
  (params (TouchedComponent :type "PrimitiveComponent Object Reference"))
  ;[0 0.003347 1] Text when Hovering
  (`SceneComponent.SetVisibility` (`self.TextRender`) true false)
  (`MeshComponent.SetOverlayMaterial` (`self.SM_Main`) "/Game/Materials/MI_YellowHighlight.MI_YellowHighlight"))

(event `self.SM_Main.OnEndCursorOver`
  (params (TouchedComponent :type "PrimitiveComponent Object Reference"))
  ;[0 0.003347 1] Text when Hovering
  (`SceneComponent.SetVisibility` (`self.TextRender`) false false)
  (`MeshComponent.SetOverlayMaterial` (`self.SM_Main`) null))

(fn `UserConstructionScript`
  (`TextRenderComponent.K2_SetText` (`self.TextRender`) (`KismetTextLibrary.Conv_NameToText` (`self.Name`))))