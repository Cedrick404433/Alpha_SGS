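; Clickable cauldron that takes the player's held ingredient, shows a count out of three and brews a potion from the mix.
; On the third, it sorts the ingredients' enum indices into a string key, so order doesn't matter.
; F_SpawnPotion matches that key against hard-coded combinations, spawning a potion or only failure smoke, then resets the slots.
; The DT_Recipes matching is disconnected old code; Tick prints debug slot contents.
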(event OnBeginCursorOver(SM_Main)
  (params (TouchedComponent :type Primitive%20Component%20Object%20Reference))
  ;[1 1 1] Sets a 'Highlight' overlay material on the Static Mesh on Cursor Over
  (Rendering|Material|SetOverlayMaterial (Variables|Default|GetSM_Main) "/Game/Materials/MI_YellowHighlight.MI_YellowHighlight" :!class /Script/Engine.MeshComponent))

(event OnClicked(SM_Main)
  (params (TouchedComponent :type Primitive%20Component%20Object%20Reference) (ButtonPressed :type Key%20Structure :default "None"))
  ;[0 0.04314 1] Cauldron interaction
  (if (Variables|/Game/Blueprints/Character/BP_Player.BP_Player_C|GetIngredientHeld? (Variables|Default|GetRef_Player))
    (Variables|/Game/Blueprints/Character/BP_Player.BP_Player_C|SetIngredientHeld? (Variables|Default|GetRef_Player) false)
    (Appearance|SetBrushfromTexture (Variables|/Game/UI/WBP_HUD.WBP_HUD_C|GetImg_ItemBox (Variables|/Game/Blueprints/Character/BP_Player.BP_Player_C|GetRef_HUD (Variables|Default|GetRef_Player))) "/Game/Textures/Blank.Blank" false)
    (Development|PrintString "Ingredient in cauldron")
    (CallFunction|ESet)
    (bind _result (Math|Integer|IncrementInt (Variables|Default|GetAddedIngredients))
      (:%20%20
        (Utilities|MSetText _result)
        (if (>= _result 3)
          (CallFunction|ECheck)
          (bind _output_get (Variables|Default|SetAddedIngredients 0))
          (Utilities|MSetText _output_get))))
    (else
      (Development|PrintString "No Ingredient Held"))))

(event OnEndCursorOver(SM_Main)
  (params (TouchedComponent :type Primitive%20Component%20Object%20Reference))
  ;[1 1 1] Sets a 'Highlight' overlay material on the Static Mesh on Cursor Over
  (Rendering|Material|SetOverlayMaterial (Variables|Default|GetSM_Main) 0 :!class /Script/Engine.MeshComponent))

(event Custom|E_SetPotionSpawn
  (bind _sm_main (Variables|Default|GetSM_Main))
  (bind _returnvalue (Transformation|GetWorldLocation _sm_main))
  ;[0 0.04314 1] Sets the spawn location for potions
  (Variables|Default|SetPotionSpawn (Math|Vector|MakeVector (.x _returnvalue) (.y _returnvalue) (+ (.z _returnvalue) 1e+01))))

(event Custom|E_SetRecipes
  ;[0 0.04314 1] Sets recipes (Not sure if needed)
  (Utilities|FlowControl|Sequence
    (:then_0
      (bind _returnvalue (Utilities|GetDataTableRow "/Game/Blueprints/Potions/DT_Recipes.DT_Recipes" "ColourCurseBlue")
        (:then
          (bind _output_get (Variables|Default|SetOut%20Row _returnvalue))
          (Variables|Recipes|SetColourCurseBlue (Utilities|Array|MakeArray (.coreingredient1 _output_get) (.coreingredient2 _output_get) (.subingredient _output_get))))))
    (:then_1
      (bind _returnvalue_2 (Utilities|GetDataTableRow "/Game/Blueprints/Potions/DT_Recipes.DT_Recipes" "ColourCurseRed")
        (:then
          (bind _output_get_2 (Variables|Default|SetOut%20Row _returnvalue_2)))))))

(event Custom|E_Set
  ;[0 0.04314 1] Sets the next empty ingredient slot
  (if (== (Variables|Ingredients|GetIngredient1) "")
    (bind _output_get (Variables|Ingredients|SetIngredient1 (Variables|/Game/Blueprints/Character/BP_Player.BP_Player_C|GetIngredientName (Variables|Default|GetRef_Player))))
    (Development|PrintString (Utilities|String|ToString(Name) _output_get))
    (elif (== (Variables|Ingredients|GetIngredient2) "")
      (bind _output_get_2 (Variables|Ingredients|SetIngredient2 (Variables|/Game/Blueprints/Character/BP_Player.BP_Player_C|GetIngredientName (Variables|Default|GetRef_Player))))
      (Development|PrintString (Utilities|String|ToString(Name) _output_get_2))
      (elif (== (Variables|Ingredients|GetIngredient3) "")
        (bind _output_get_3 (Variables|Ingredients|SetIngredient3 (Variables|/Game/Blueprints/Character/BP_Player.BP_Player_C|GetIngredientName (Variables|Default|GetRef_Player))))
        (Development|PrintString (Utilities|String|ToString(Name) _output_get_3))
        ;[0 1 0.0832] Uses loops and arrays to get the enum position of the three selected ingredients from enum_ingredients and put them into an integer array ready to be sorted.
        (Variables|Default|SetintTempArray (Utilities|Array|MakeArray 0 0 0))
        (bind _output_get_4 (Variables|Default|SetingredientArray (Utilities|Array|MakeArray (Variables|Ingredients|GetIngredient1) (Variables|Ingredients|GetIngredient2) (Variables|Ingredients|GetIngredient3))))
        (for (_array_element _array_index) _output_get_4
          (bind _enumvalue (|ForEachenum_ingredients)
            (:LoopBody
              (if (== _array_element (Utilities|String|StringToName (Utilities|String|EnumtoString _enumvalue)))
                (Utilities|Array|SetArrayElem (Variables|Default|GetintTempArray) _array_index (Math|Conversions|ToInteger(Byte) _enumvalue) true)))))
        ;[0 1 0.0832] Sorts the items in the integer array into ascending order, then turns them into a 3 digit string.
        (Class|KismetArrayLibrary|SortIntArray (Variables|Default|GetintTempArray))
        (Variables|Default|SetstringTemp "")
        (for _array_element_2 (Variables|Default|GetintTempArray)
          (bind _output_get_5 (Variables|Default|SetstringTemp (Utilities|String|Append (Variables|Default|GetstringTemp) (Utilities|String|ToString(Integer) _array_element_2))))
          (Development|PrintString _output_get_5))
        (CallFunction|FSpawnPotion)))))

(event Custom|E_Check
  ;[1 0.4653 0] Old Code
)

(event Custom|E_Break
  ;[1 0.4653 0] Old Code
  (Utilities|Array|ForEachLoopwithBreak (stale _outrownames)) ; enters at Break
)

(event EventBeginPlay
  ;[0 0.04314 1] Cast and setup
  (bind _asbp_player (Utilities|Casting|CastToBP_Player (Game|GetPlayerCharacter 0)))
  (Variables|Default|SetRef_Player _asbp_player)
  (Development|PrintString "Character" true true "(R=0.000000,G=1.000000,B=0.120832,A=1.000000)")
  (CallFunction|ESetRecipes)
  (CallFunction|ESetPotionSpawn))

(event EventTick
  (params (DeltaSeconds :type Float%20%28single-precision%29))
  ;[1 0 0.843] Debug to show current ingredients
  (Development|PrintString (Utilities|String|ToString(Name) (Variables|Ingredients|GetIngredient1)) true true "(R=1.000000,G=0.000000,B=0.627451,A=1.000000)" 0.0)
  (Development|PrintString (Utilities|String|ToString(Name) (Variables|Ingredients|GetIngredient2)) true true "(R=1.000000,G=0.000000,B=0.627451,A=1.000000)" 0.0)
  (Development|PrintString (Utilities|String|ToString(Name) (Variables|Ingredients|GetIngredient3)) true true "(R=1.000000,G=0.000000,B=0.627451,A=1.000000)" 0.0))

(fn ConstructionScript)

(fn FReset
  (Variables|Ingredients|SetCheck1 false)
  (Variables|Ingredients|SetCheck2 false)
  (Variables|Ingredients|SetCheck3 false)
  (Variables|Ingredients|SetIngredient1 "")
  (Variables|Ingredients|SetIngredient2 "")
  (Variables|Ingredients|SetIngredient3 "")
  (return))

(fn FSpawnPotion
  (bind _sm_main (Variables|Default|GetSM_Main))
  (bind _returnvalue (Transformation|GetWorldLocation _sm_main))
  (bind _returnvalue_2 (+ _returnvalue "0.000000,0.000000,-35.000000"))
  ;[0 0.04314 1] Spawns the corresponding potion
  (if (== (Utilities|String|StringToName (Variables|Default|GetstringTemp)) "012")
    (Game|SpawnActorfromClass "/Game/Blueprints/Potions/BPC_ColourPotionBlue.BPC_ColourPotionBlue_C" (Math|Transform|MakeTransform (Variables|Default|GetPotionSpawn) "0, 0, 0" "1.000000,1.000000,1.000000") "Undefined" "MultiplyWithRoot" 0 0)
    (Variables|/Game/Blueprints/Character/BP_Player.BP_Player_C|SetPotionHeld (Variables|Default|GetRef_Player) (Variables|Default|GetPotionName) :!label _label)
    (CallFunction|FReset)
    ;[1 1 1] Spawns a Niagara FX depending on the mix of Ingredients
    (Niagara|SpawnSystematLocation "/Game/VFX/NS_Smoke.NS_Smoke" _returnvalue_2)
    (elif (== (Utilities|String|StringToName (Variables|Default|GetstringTemp)) "013")
      (Game|SpawnActorfromClass "/Game/Blueprints/Potions/BPC_ColourPotionRed.BPC_ColourPotionRed_C" (Math|Transform|MakeTransform (Variables|Default|GetPotionSpawn) "0, 0, 0" "1.000000,1.000000,1.000000") "Undefined" "MultiplyWithRoot" 0 0)
      (goto _label)
      (elif (== (Utilities|String|StringToName (Variables|Default|GetstringTemp)) "456")
        (Game|SpawnActorfromClass "/Game/Blueprints/Potions/BPC_GlowPotion.BPC_GlowPotion_C" (Math|Transform|MakeTransform (Variables|Default|GetPotionSpawn) "0, 0, 0" "1.000000,1.000000,1.000000") "Undefined" "MultiplyWithRoot" 0 0)
        (goto _label)
        (elif (== (Utilities|String|StringToName (Variables|Default|GetstringTemp)) "789")
          (Game|SpawnActorfromClass "/Game/Blueprints/Potions/BPC_GiantPotionHand.BPC_GiantPotionHand_C" (Math|Transform|MakeTransform (Variables|Default|GetPotionSpawn) "0, 0, 0" "1.000000,1.000000,1.000000") "Undefined" "MultiplyWithRoot" 0 0)
          (goto _label)
          (elif (== (Utilities|String|StringToName (Variables|Default|GetstringTemp)) "7810")
            (Game|SpawnActorfromClass "/Game/Blueprints/Potions/BPC_GiantPotionHead.BPC_GiantPotionHead_C" (Math|Transform|MakeTransform (Variables|Default|GetPotionSpawn) "0, 0, 0" "1.000000,1.000000,1.000000") "Undefined" "MultiplyWithRoot" 0 0)
            (goto _label)
            (else
              (CallFunction|FReset)
              (Niagara|SpawnSystematLocation "/Game/VFX/NS_Inc_Smoke.NS_Inc_Smoke" _returnvalue_2))))))))