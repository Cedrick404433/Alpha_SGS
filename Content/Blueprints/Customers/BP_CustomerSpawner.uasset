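; BP_CustomerSpawner keeps a customer in the level by spawning a BP_Customer whenever none exists.
; On BeginPlay it starts a looping one-second timer that searches the world for any BP_Customer actor.
; When the search finds none, it spawns one at the SpawnPoint transform, ignoring collisions, and prints a debug message.
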(event `self.ReceiveBeginPlay`
  (`KismetSystemLibrary.K2_SetTimerDelegate` (delegate `E_SpawnCheck`) 1.0 true))

(event `E_SpawnCheck`
  (bind _outactors (`GameplayStatics.GetAllActorsOfClass` "/Game/Blueprints/Customers/BP_Customer.BP_Customer_C"))
  (if (not (`KismetArrayLibrary.Array_IsValidIndex` _outactors))
    (`self.E_SpawnCustomer`)))

(event `E_SpawnCustomer`
  ;[1 1 1] Comment
  (`|SpawnActorFromClass` "/Game/Blueprints/Customers/BP_Customer.BP_Customer_C" (`SceneComponent.K2_GetComponentToWorld` (`self.SpawnPoint`)) "AlwaysSpawn" "MultiplyWithRoot" null null)
  (`KismetSystemLibrary.PrintString` "Customer Spawned" true true (struct :`G` 1.0 :`B` 0.132018 :`A` 1.0)))

(fn `UserConstructionScript`)