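; Customer actor that arrives with a random curse and pays gold when clicked with the matching potion.
; BeginPlay draws a DT_Curses row to set the cube material and curse text, and starts a looping timer, apparently for the leave countdown.
; Clicks compare the curse name to BP_Cauldron's StringTemp, then award gold, clear it and destroy the customer.
; Hover toggles a material glow; E is a debug toggle, and dialogue logic is largely unwired.
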(event `self.ReceiveBeginPlay`
  (`|ExecutionSequence`
    (:`then_0`
      (bind _asbp_player (cast `/Game/Blueprints/Character/BP_Player` (`GameplayStatics.GetPlayerCharacter` 0)))
      (set `self.Ref_Character` _asbp_player)
      (bind _asgm_main (cast `/Game/Blueprints/Character/GM_Main` (`GameplayStatics.GetGameMode`)))
      (set `self.Ref_Gamemode` _asgm_main)
      ;[1 1 1] Door Bell SFX
      (`GameplayStatics.PlaySound2D` "/Game/Placeholder/Audio/SW_DoorBell.SW_DoorBell" 1.0 1.0 0.0 null null)
      (set `self.IsSicknessVisible?` false)
      (bind _outrownames (`DataTableFunctionLibrary.GetDataTableRowNames` "/Game/Blueprints/Curses/DT_Curses.DT_Curses"))
      (set `self.Curses` _outrownames)
      (`self.E_RandomCurse`)
      (`KismetSystemLibrary.K2_SetTimerDelegate` (`|CreateDelegate` :!event `E_Timer`) 1.0 true))))

(event `E_UpdateDialogue`)

(event `self.Cube.OnClicked`
  (params (TouchedComponent :type "PrimitiveComponent Object Reference") (ButtonPressed :type "Key Structure"))
  (bind _ref_gamemode (`self.Ref_Gamemode`))
  ;[1 1 0] Attempted dialogue system for customer when interacted
  (if (`/Game/Blueprints/Character/BP_Player.IsPotionHeld?` (`self.Ref_Character`))
    ;[0.6719 0 0] Takes stringTemp from bp_cauldron and compares it to the name in STR_Curses to check if the correct potion is held.
    (bind _returnvalue (`GameplayStatics.GetActorOfClass` "/Game/Blueprints/Cauldron/BP_Cauldron.BP_Cauldron_C"))
    (bind _stringtemp (`/Game/Blueprints/Cauldron/BP_Cauldron.stringTemp` _returnvalue))
    (`KismetSystemLibrary.PrintString` _stringtemp)
    (if (== (`.Name_2_DBF5305C4BA57987632E42AC02E95A92` (break `/Game/Blueprints/Curses/STR_Curses` (`self.STR_Curses`))) _stringtemp)
      (`/Engine/EditorBlueprintResources/StandardMacros.DoOnce` false
        (:`Completed`
          (`KismetSystemLibrary.PrintString` "Thank You!" true true (struct :`G` 1.0 :`A` 1.0))
          (set `/Game/Blueprints/Character/GM_Main.Gold` (+ (`/Game/Blueprints/Character/GM_Main.Gold` _ref_gamemode) (`self.GoldIncome`)) _ref_gamemode)
          (`/Game/UI/WBP_HUD.E_UpdateGold` (`/Game/Blueprints/Character/BP_Player.Ref_HUD` (`self.Ref_Character`)))
          ;[0.6719 0 0] Resets stringTemp to nothing to fix issue where the game remembered the last made potion.
          (bind _returnvalue_2 (`GameplayStatics.GetActorOfClass` "/Game/Blueprints/Cauldron/BP_Cauldron.BP_Cauldron_C"))
          (set `/Game/Blueprints/Cauldron/BP_Cauldron.stringTemp` "" _returnvalue_2)
          (`KismetSystemLibrary.Delay` 1.0)
          (`self.K2_DestroyActor`)))
      (else
        (`KismetSystemLibrary.PrintString` "Wrong!" true true (struct :`R` 1.0 :`A` 1.0))))))

(event `E_UpdateScene`
  (params (Enum_Dialogue :type "/Game/Blueprints/Character/Dialogue/Enum_Dialogue Enum" :default "NewEnumerator0"))
  (bind _output_get (set `self.Enum_Dialogue` Enum_Dialogue))
  ;[1 1 0] Attempted dialogue system for customer when interacted
  (bind _returnvalue (`|GetDataTableRow` "/Game/Blueprints/Character/Dialogue/DT_Dialogue.DT_Dialogue" (select `/Game/Blueprints/Character/Dialogue/Enum_Dialogue` _output_get :`NewEnumerator0` "Initial" :`NewEnumerator1` "Sickness" :`NewEnumerator2` "Potion" :`NewEnumerator3` "Completed" :`NewEnumerator4` "Failed" :!type "Name"))
    (:`then`
      (set `self.CurrentDialogue` _returnvalue))))

(event `E_RandomCurse`
  (bind _returnvalue (`|GetDataTableRow` "/Game/Blueprints/Curses/DT_Curses.DT_Curses" (`KismetArrayLibrary.Array_Random` (`self.Curses`)))
    (:`then`
      (bind _output_get (set `self.STR_Curses` _returnvalue))
      (`self.F_CurseName` (`KismetStringLibrary.Conv_StringToName` (break `/Game/Blueprints/Curses/STR_Curses` _output_get)))
      (`PrimitiveComponent.SetMaterial` (`self.Cube`) 0 (`.Material_10_7C094A99441F980B511C1E9FBB7C0048` (break `/Game/Blueprints/Curses/STR_Curses` _output_get))))))

(event `E_Timer`
  (if (<= (`self.Time`) 1)
    (`KismetSystemLibrary.PrintString` "Customer Left!" true true (struct :`R` 1.0 :`A` 1.0))
    (`self.K2_DestroyActor`)
    (else
      (bind _result (`/Engine/EditorBlueprintResources/StandardMacros.DecrementInt` (`self.Time`))
        (:`  `
          (set `self.Time` _result))))))

(event `Key|E`
  (params (Key :type "Key Structure"))
  ;[0 1 1] Activate "Potion Held" Debug
  (:`Pressed`
    (`/Engine/EditorBlueprintResources/StandardMacros.FlipFlop`
      (:`A`
        (bind _output_get (set `self.IsHoldingPotion?` true))
        (`KismetSystemLibrary.PrintString` (`KismetStringLibrary.Conv_BoolToString` _output_get)))
      (:`B`
        (bind _output_get_2 (set `self.IsHoldingPotion?` false))
        (`KismetSystemLibrary.PrintString` (`KismetStringLibrary.Conv_BoolToString` _output_get_2))))))

(event `self.Cube.OnBeginCursorOver`
  (params (TouchedComponent :type "PrimitiveComponent Object Reference"))
  ;[1 1 1] Glow Effect on Cursor Hover
  (`MeshComponent.SetScalarParameterValueOnMaterials` (`self.SKM_Customer`) "Interacted" 1.0)
  (`MeshComponent.SetScalarParameterValueOnMaterials` (`self.Cube`) "Interacted" 1.0))

(event `self.Cube.OnEndCursorOver`
  (params (TouchedComponent :type "PrimitiveComponent Object Reference"))
  ;[1 1 1] Glow Effect on Cursor Hover
  (`MeshComponent.SetScalarParameterValueOnMaterials` (`self.SKM_Customer`) "Interacted" 0.0)
  (`MeshComponent.SetScalarParameterValueOnMaterials` (`self.Cube`) "Interacted" 0.0))

(fn `F_CurseName`
  (params (Name :type Name))
  (locals (C_BlueGlow :type Text :default "NSLOCTEXT(\"[BA127D849D9C6054446D48CC0FB959BE]\", \"6C2062BC4164B86C5EFFA79962DE6D36\", \"Blue Colour\")") (C_RedGlow :type Text :default "NSLOCTEXT(\"[BA127D849D9C6054446D48CC0FB959BE]\", \"E05B393E49016A7902055A9DC5D65764\", \"Red Colour\")") (C_Glow :type Text :default "NSLOCTEXT(\"[BA127D849D9C6054446D48CC0FB959BE]\", \"278D8BC24D2FD3861A098E8F057AB6E2\", \"Glow\")") (C_GiantHand :type Text :default "NSLOCTEXT(\"[BA127D849D9C6054446D48CC0FB959BE]\", \"89363D87424EC7A1C42B69B05CD940A7\", \"Giant Hand\")") (C_GiantHead :type Text :default "NSLOCTEXT(\"[BA127D849D9C6054446D48CC0FB959BE]\", \"B2C4DF0F435644610A736487AC49BBE9\", \"Giant Head\")"))
  (if (== "012" Name)
    (`TextRenderComponent.K2_SetText` (`self.TextRender`) (`local.C_BlueGlow`))
    (elif (== "013" Name)
      (`TextRenderComponent.K2_SetText` (`self.TextRender`) (`local.C_RedGlow`))
      (elif (== "456" Name)
        (`TextRenderComponent.K2_SetText` (`self.TextRender`) (`local.C_Glow`))
        (elif (== "789" Name)
          (`TextRenderComponent.K2_SetText` (`self.TextRender`) (`local.C_GiantHand`))
          (elif (== "7810" Name)
            (`TextRenderComponent.K2_SetText` (`self.TextRender`) (`local.C_GiantHead`))))))))

(fn `UserConstructionScript`)